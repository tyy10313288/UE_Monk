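; BP_CopyScriptPlace is the interaction spot for the scripture-copying minigame.
; Its Box overlap registers the actor as CopyScript on the player's BP_ThirdPersonCharacter and clears it when the player leaves.
; OnInteractingCopyScript blends the player's view to the owner of ScriptCam, enables the mouse cursor with click and hover events, and adds a WBP_Copy widget to the viewport.
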(event `self.Box.OnComponentBeginOverlap`
  (params (OverlappedComponent :type "PrimitiveComponent Object Reference") (OtherActor :type "Actor Object Reference") (OtherComp :type "PrimitiveComponent Object Reference") (OtherBodyIndex :type Integer) (bFromSweep :type Boolean) (SweepResult :type "HitResult Structure (by ref)"))
  (if (== OtherActor (`GameplayStatics.GetPlayerPawn` 0))
    (bind _asbp_third_person_character (cast `/Game/ThirdPerson/Blueprints/BP_ThirdPersonCharacter` OtherActor))
    (set `/Game/ThirdPerson/Blueprints/BP_ThirdPersonCharacter.CopyScript` self _asbp_third_person_character)
    (set `self.As BP Third Person Character_0` _asbp_third_person_character)))

(event `self.Box.OnComponentEndOverlap`
  (params (OverlappedComponent :type "PrimitiveComponent Object Reference") (OtherActor :type "Actor Object Reference") (OtherComp :type "PrimitiveComponent Object Reference") (OtherBodyIndex :type Integer))
  (if (== OtherActor (`GameplayStatics.GetPlayerPawn` 0))
    (bind _asbp_third_person_character (cast `/Game/ThirdPerson/Blueprints/BP_ThirdPersonCharacter` OtherActor))
    (set `/Game/ThirdPerson/Blueprints/BP_ThirdPersonCharacter.CopyScript` null _asbp_third_person_character)
    (set `self.As BP Third Person Character_1` _asbp_third_person_character)))

(event `OnInteractingCopyScript`
  (bind _returnvalue (`GameplayStatics.GetPlayerController` 0))
  (`PlayerController.SetViewTargetWithBlend` (`GameplayStatics.GetPlayerController` 0) (`ActorComponent.GetOwner` (`self.ScriptCam`)) 0.0 "VTBlend_Linear" 0.0 false)
  (`|ExecutionSequence`
    (:`then_0`
      (bind _output_get (set `PlayerController.bShowMouseCursor` true _returnvalue))
      (bind _output_get_2 (set `PlayerController.bEnableClickEvents` _output_get _returnvalue))
      (set `PlayerController.bEnableMouseOverEvents` _output_get_2 _returnvalue))
    (:`then_1`
      (bind _returnvalue_2 (`|CreateWidget` "/Game/MiniGame/CopyScriptures/WBP_Copy.WBP_Copy_C"))
      (bind _output_get_3 (set `self.Copy widget` _returnvalue_2))
      (`UserWidget.AddToViewport` _output_get_3 0))))

(fn `UserConstructionScript`)