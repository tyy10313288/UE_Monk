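; BP_WoodenFish is the interactable actor for a wooden fish minigame, registering itself on the third-person character while the player overlaps its box.
; Interaction switches the view to this actor's camera, shows the cursor and opens the WBP_WoodenFish widget.
; Kok animates the stick's hit with a timeline-driven roll.
; BackToPlayerCam restores player view and walking once BP_Spline reaches its spawn count, and separately sets a Testing2 flag for high scores.
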(event `self.Box.OnComponentBeginOverlap`
  (params (OverlappedComponent :type "PrimitiveComponent Object Reference") (OtherActor :type "Actor Object Reference") (OtherComp :type "PrimitiveComponent Object Reference") (OtherBodyIndex :type Integer) (bFromSweep :type Boolean) (SweepResult :type "HitResult Structure (by ref)"))
  (if (== OtherActor (`GameplayStatics.GetPlayerPawn` 0))
    (bind _asbp_third_person_character (cast `/Game/ThirdPerson/Blueprints/BP_ThirdPersonCharacter` OtherActor))
    (set `/Game/ThirdPerson/Blueprints/BP_ThirdPersonCharacter.WoodenFishActor` self _asbp_third_person_character)
    (set `self.Player Ref` _asbp_third_person_character)))

(event `self.Box.OnComponentEndOverlap`
  (params (OverlappedComponent :type "PrimitiveComponent Object Reference") (OtherActor :type "Actor Object Reference") (OtherComp :type "PrimitiveComponent Object Reference") (OtherBodyIndex :type Integer))
  (if (== OtherActor (`GameplayStatics.GetPlayerPawn` 0))
    (bind _asbp_third_person_character (cast `/Game/ThirdPerson/Blueprints/BP_ThirdPersonCharacter` OtherActor))
    (set `/Game/ThirdPerson/Blueprints/BP_ThirdPersonCharacter.WoodenFishActor` null _asbp_third_person_character)
    (set `self.Player Ref` _asbp_third_person_character)))

(event `OnInteractingWoodenFish`
  (bind _returnvalue (`GameplayStatics.GetPlayerController` 0))
  ; Getting Interection
  (`PlayerController.SetViewTargetWithBlend` (`GameplayStatics.GetPlayerController` 0) (`ActorComponent.GetOwner` (`self.WoodenFishCam`)) 0.0 "VTBlend_Linear" 0.0 false)
  (`|ExecutionSequence`
    (:`then_0`
      (bind _output_get (set `PlayerController.bShowMouseCursor` true _returnvalue))
      (bind _output_get_2 (set `PlayerController.bEnableClickEvents` _output_get _returnvalue))
      (set `PlayerController.bEnableMouseOverEvents` _output_get_2 _returnvalue))
    (:`then_1`
      (bind _returnvalue_2 (`|CreateWidget` "/Game/MiniGame/WoodenFish/WBP_WoodenFish.WBP_WoodenFish_C"))
      (bind _output_get_3 (set `self.WoodenFishStartPanel` _returnvalue_2))
      (`UserWidget.AddToViewport` _output_get_3 0))
    (:`then_2`
      (set `self.PlayingWoodenFish` true))))

(event `Kok`
  ; Hitting Action
  (bind (_direction _kok) (`Timeline|タイムライン` :!via `PlayFromStart`)
    (:`Update`
      (`SceneComponent.K2_SetRelativeRotation` (`self.Stick`) (`KismetMathLibrary.MakeRotator` _kok) false false))))

(event `BackToPlayerCam`
  (bind _returnvalue (`GameplayStatics.GetPlayerController` 0))
  (bind _asbp_third_person_character (cast `/Game/ThirdPerson/Blueprints/BP_ThirdPersonCharacter` (`GameplayStatics.GetPlayerPawn` 0) :!pure true))
  (`|ExecutionSequence`
    (:`then_0`
      (bind _returnvalue_2 (`GameplayStatics.GetActorOfClass` "/Game/MiniGame/WoodenFish/BP_Spline.BP_Spline_C"))
      (if (== (`/Game/MiniGame/WoodenFish/BP_Spline.SpawnCount` _returnvalue_2) 10.0)
        (bind _output_get (set `PlayerController.bShowMouseCursor` false _returnvalue))
        (bind _output_get_2 (set `PlayerController.bEnableClickEvents` _output_get _returnvalue))
        (set `PlayerController.bEnableMouseOverEvents` _output_get_2 _returnvalue)
        (`PlayerController.SetViewTargetWithBlend` _returnvalue (`ActorComponent.GetOwner` (`/Game/ThirdPerson/Blueprints/BP_ThirdPersonCharacter.FollowCamera` _asbp_third_person_character)) 0.0 "VTBlend_Linear" 0.0 false)
        (`CharacterMovementComponent.SetMovementMode` (`Character.CharacterMovement` _asbp_third_person_character) "MOVE_Walking" 0)
        (set `self.PlayingWoodenFish` false)))
    (:`then_1`
      (if (> (`/Game/ThirdPerson/Blueprints/BP_ThirdPersonCharacter.WoodenFishPoint` (`self.Player Ref`)) 8)
        (set `self.testing2` true)))))

(fn `UserConstructionScript`)