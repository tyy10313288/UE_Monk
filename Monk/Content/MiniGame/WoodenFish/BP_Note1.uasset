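; BP_Note1 is a note actor for the WoodenFish rhythm minigame that travels along a spline path.
; On BeginPlay it caches the BP_Spline actor found in the level.
; Its moving event plays a timeline at a rate of 1/TimeToComplete, mapping the track to distance along the spline.
; Each update sets world position and rotation from the spline, with a fixed reduced scale.
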(event `self.ReceiveBeginPlay`
  (bind _returnvalue (`GameplayStatics.GetActorOfClass` "/Game/MiniGame/WoodenFish/BP_Spline.BP_Spline_C"))
  (set `self.rhythm` _returnvalue))

(event `moving`
  (bind _spline (`/Game/MiniGame/WoodenFish/BP_Spline.Spline` (`self.rhythm`)))
  (`TimelineComponent.SetPlayRate` (`self.タイムライン`) (/ 1.0 (`self.TimeToComplete`)))
  (bind (_direction `_新規track_0`) (`Timeline|タイムライン` :!via `PlayFromStart`)
    (:`Update`
      (bind _returnvalue (`KismetMathLibrary.Lerp` 0.0 (`SplineComponent.GetSplineLength` (`/Game/MiniGame/WoodenFish/BP_Spline.Spline` (`self.rhythm`))) `_新規track_0`))
      (`self.K2_SetActorTransform` (`KismetMathLibrary.MakeTransform` (`SplineComponent.GetLocationAtDistanceAlongSpline` _spline _returnvalue "World") (`SplineComponent.GetRotationAtDistanceAlongSpline` _spline _returnvalue "World") (0.2 0.2 0.2))))))

(fn `UserConstructionScript`)