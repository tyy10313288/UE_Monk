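; BP_TalkChara is the monk NPC (方丈) in the Monk minigame, holding name, icon and lines inviting the player to train before ordination.
; A Box overlap registers or clears it as the player character's TalkCharaActor.
; TalkToChara plays a Rotation timeline that lerps the actor toward the player and sets Talking.
; Both overlaps set PlayerRef from the end-overlap cast, and the mouse-cursor setup never runs.
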(event `self.ReceiveBeginPlay`
  (set `self.CharaSpec` (make `/Game/MiniGame/Monk/Struct_CharaSpec` "方丈" (`|MakeArray` "你想出家嗎?" "為了確認你的真心..." "先進行修行吧!") "/Game/Asset/OldMonk/MonkIcon.MonkIcon")))

(event `self.Box.OnComponentBeginOverlap`
  (params (OverlappedComponent :type "PrimitiveComponent Object Reference") (OtherActor :type "Actor Object Reference") (OtherComp :type "PrimitiveComponent Object Reference") (OtherBodyIndex :type Integer) (bFromSweep :type Boolean) (SweepResult :type "HitResult Structure (by ref)"))
  (if (== OtherActor (`GameplayStatics.GetPlayerCharacter` 0))
    (bind _asbp_third_person_character (cast `/Game/ThirdPerson/Blueprints/BP_ThirdPersonCharacter` OtherActor))
    (set `/Game/ThirdPerson/Blueprints/BP_ThirdPersonCharacter.TalkCharaActor` self _asbp_third_person_character)
    (set `self.PlayerRef` (stale `self.Box.OnComponentEndOverlap` _asbp_third_person_character) :!label _label)))

(event `self.Box.OnComponentEndOverlap`
  (params (OverlappedComponent :type "PrimitiveComponent Object Reference") (OtherActor :type "Actor Object Reference") (OtherComp :type "PrimitiveComponent Object Reference") (OtherBodyIndex :type Integer))
  (if (== (`GameplayStatics.GetPlayerCharacter` 0) OtherActor)
    (bind _asbp_third_person_character (cast `/Game/ThirdPerson/Blueprints/BP_ThirdPersonCharacter` OtherActor))
    (set `/Game/ThirdPerson/Blueprints/BP_ThirdPersonCharacter.TalkCharaActor` null _asbp_third_person_character)
    (goto _label)))

(event `TalkToChara`
  (`|ExecutionSequence`
    (:`then_0`
      (bind (_direction _alpha) (`Timeline|Rotation`)
        (:`Update`
          (`self.K2_SetActorRotation` (`KismetMathLibrary.RLerp` (`self.K2_GetActorRotation`) (`KismetMathLibrary.FindLookAtRotation` (`self.K2_GetActorLocation`) (`self.K2_GetActorLocation` (`GameplayStatics.GetPlayerCharacter` 0))) _alpha))
          (set `self.Talking` true))))))

(fn `UserConstructionScript`)