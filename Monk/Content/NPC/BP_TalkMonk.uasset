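; BP_TalkMonk is the monk NPC who invites the player to train for priesthood and delivers the game's ending.
; BeginPlay sets the dialogue and binds SetTalkState to a talk-state check.
; SetTalkState reads the player's CS and WF flags: unfinished repeats the intro, while finished picks success or failure dialogue.
; After a delay, it plays EndSequence, shows the cursor and reveals the ending widget with the result.
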(event `self.ReceiveBeginPlay`
  (set `self.CharaSpec` (make `/Game/NPC/Struct_CharaSpec` "禅師" (`|MakeArray` "僧侶になりたいですか？" "あなたの誠意を確かめるために…" "まずは修行をしてみましょう！") "/Game/Asset/OldMonk/MonkIcon.MonkIcon"))
  (add `self.CheckTalkState` (delegate `SetTalkState`)))

(event `SetTalkState`
  (bind _returnvalue (`GameplayStatics.GetActorOfClass` "/Game/ThirdPerson/Blueprints/BP_ThirdPersonCharacter.BP_ThirdPersonCharacter_C"))
  (if (and (`/Game/ThirdPerson/Blueprints/BP_ThirdPersonCharacter.CSfinshed` _returnvalue) (`/Game/ThirdPerson/Blueprints/BP_ThirdPersonCharacter.WFfinshed` _returnvalue))
    (if (and (`/Game/ThirdPerson/Blueprints/BP_ThirdPersonCharacter.CSsucees` _returnvalue) (`/Game/ThirdPerson/Blueprints/BP_ThirdPersonCharacter.WFsucees` _returnvalue))
      (setmembers `/Game/NPC/Struct_CharaSpec` :`StructRef` (`self.CharaSpec`) :`Talk` (`|MakeArray` "修行完了したね、えらい！"))
      (set `self.GameClear` true)
      (else
        (setmembers `/Game/NPC/Struct_CharaSpec` :`StructRef` (`self.CharaSpec`) :`Talk` (`|MakeArray` "修行失敗したね、残念。"))
        (set `self.GameClear` false)))
    (`KismetSystemLibrary.Delay` 2.0)
    (bind _outactor (`LevelSequencePlayer.CreateLevelSequencePlayer` (`self.EndSequence`)))
    (`MovieSceneSequencePlayer.Play` (`LevelSequenceActor.SequencePlayer` _outactor))
    (set `PlayerController.bShowMouseCursor` true (`GameplayStatics.GetPlayerController` 0))
    (`self.SetEndingWBPvisible`)
    (else
      (setmembers `/Game/NPC/Struct_CharaSpec` :`StructRef` (`self.CharaSpec`) :`Talk` (`|MakeArray` "僧侶になりたいですか？" "あなたの誠意を確かめるために…" "まずは修行をしてみましょう！")))))

(event `SetEndingWBPvisible`
  (bind _wbp_ending (`/Game/ThirdPerson/Blueprints/BP_ThirdPersonCharacter.WBP Ending` (`self.Player Ref`)))
  ; play ending sequence and show the ending word
  (`Widget.SetVisibility` (`/Game/MiniGame/WBP_Ending.Quit` (`/Game/ThirdPerson/Blueprints/BP_ThirdPersonCharacter.WBP Ending` (stale `SetTalkState` _returnvalue))) "Visible")
  (`Widget.SetVisibility` (`/Game/MiniGame/WBP_Ending.Title` (`/Game/ThirdPerson/Blueprints/BP_ThirdPersonCharacter.WBP Ending` (stale `SetTalkState` _returnvalue))) "Visible")
  (set `self.PlayEnding` true)
  (if (`self.GameClear`)
    (set `/Game/MiniGame/WBP_Ending.textend` (`KismetTextLibrary.Conv_TextToString` (`|FormatText` "修行成功")) _wbp_ending)
    (else
      (set `/Game/MiniGame/WBP_Ending.textend` (`KismetTextLibrary.Conv_TextToString` (`|FormatText` "修行失敗")) _wbp_ending))))

(fn `UserConstructionScript`
  (`parent.UserConstructionScript`))