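; BP_TalkMonk is the Zen master NPC of the conversation system, who invites the player to train as a monk.
; BeginPlay fills CharaSpec with name, dialogue and icon, then binds SetTalkState to CheckTalkState.
; SetTalkState checks the player character's CSsucees and WFsucees flags to choose the training prompt or praise.
; When both are set, it also sets GameClear and plays a level sequence after a short delay.
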(event `self.ReceiveBeginPlay`
  (set `self.CharaSpec` (make `/Game/ConversationSystem/Struct_CharaSpec` "禅師" (`|MakeArray` "僧侶になりたいですか？" "あなたの誠意を確かめるために…" "まずは修行をしてみましょう！") "/Game/Asset/OldMonk/MonkIcon.MonkIcon"))
  (add `self.CheckTalkState` (delegate `SetTalkState`)))

(event `SetTalkState`
  (bind _returnvalue (`GameplayStatics.GetActorOfClass` "/Game/ThirdPerson/Blueprints/BP_ThirdPersonCharacter.BP_ThirdPersonCharacter_C"))
  (if (and (`/Game/ThirdPerson/Blueprints/BP_ThirdPersonCharacter.CSsucees` _returnvalue) (`/Game/ThirdPerson/Blueprints/BP_ThirdPersonCharacter.WFsucees` _returnvalue))
    (setmembers `/Game/ConversationSystem/Struct_CharaSpec` :`StructRef` (`self.CharaSpec`) :`Talk` (`|MakeArray` "修行完了したね、えらい！"))
    (set `self.GameClear` true)
    (`KismetSystemLibrary.Delay` 2.0)
    (bind _outactor (`LevelSequencePlayer.CreateLevelSequencePlayer` (`self.NewVar`)))
    (`MovieSceneSequencePlayer.Play` (`LevelSequenceActor.SequencePlayer` _outactor))
    (else
      (setmembers `/Game/ConversationSystem/Struct_CharaSpec` :`StructRef` (`self.CharaSpec`) :`Talk` (`|MakeArray` "僧侶になりたいですか？" "あなたの誠意を確かめるために…" "まずは修行をしてみましょう！")))))

(fn `UserConstructionScript`
  (`parent.UserConstructionScript`))